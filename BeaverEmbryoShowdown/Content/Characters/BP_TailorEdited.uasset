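; BP_TailorEdited is a playable gamepad fighter in a two-player match, whose death shows the Player 2 victory screen and pauses the game.
; Axis inputs drive world-relative movement and lerped facing, while shoulder and trigger set slap and slam flags on the AnimBP.
; Punch and Slam events apply damage through forward capsule traces.
; AnyDamage reduces CurrentHealth, separate from the Health used by CalculateHealth and CalculateDead.
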(event `InputAxis|LookUp`
  (params (AxisValue :type "Float (single-precision)"))
  ;[1 1 1] Rotation
  (bind _returnvalue (`KismetMathLibrary.MakeVector` AxisValue (stale `InputAxis|LookRight` AxisValue)))
  (if (> (`KismetMathLibrary.VSize` _returnvalue) 0.25) :!label _label
    (`Controller.SetControlRotation` (`self.GetController`) (`KismetMathLibrary.RLerp` (`self.K2_GetActorRotation`) (`KismetMathLibrary.Conv_VectorToRotator` _returnvalue) 0.4 true))))

(event `InputAxis|MoveUp`
  (params (AxisValue :type "Float (single-precision)"))
  ;[1 1 1] Movement
  (set `CharacterMovementComponent.MaxWalkSpeed` (`self.Mvmt Speed`) (`self.CharacterMovement`))
  (`self.AddMovementInput` (1.0 0.0 0.0) AxisValue))

(event `InputAxis|LookRight`
  (params (AxisValue :type "Float (single-precision)"))
  ;[1 1 1] Rotation
  (goto _label))

(event `InputAxis|MoveRight`
  (params (AxisValue :type "Float (single-precision)"))
  ;[1 1 1] Movement
  (set `CharacterMovementComponent.MaxWalkSpeed` (`self.Mvmt Speed`) (`self.CharacterMovement`))
  (`self.AddMovementInput` (0.0 1.0 0.0) AxisValue))

(event `Key|Gamepad_RightShoulder`
  (params (Key :type "Key Structure"))
  (bind _returnvalue (`SkeletalMeshComponent.GetAnimInstance` (`self.Mesh`)))
  ;[1 1 1] Attack Animations
  (:`Pressed`
    (bind _asabp_tailor_edited (cast `/Game/Characters/ABP_TailorEdited` _returnvalue))
    (set `/Game/Characters/ABP_TailorEdited.CanSlap` true _asabp_tailor_edited))
  (:`Released`
    (bind _asabp_tailor_edited_2 (cast `/Game/Characters/ABP_TailorEdited` _returnvalue))
    (set `/Game/Characters/ABP_TailorEdited.CanSlap` false _asabp_tailor_edited_2)))

(event `Key|Gamepad_RightTrigger`
  (params (Key :type "Key Structure"))
  (bind _returnvalue (`SkeletalMeshComponent.GetAnimInstance` (`self.Mesh`)))
  ;[1 1 1] Attack Animations
  (:`Pressed`
    (bind _asabp_tailor_edited (cast `/Game/Characters/ABP_TailorEdited` _returnvalue))
    (set `/Game/Characters/ABP_TailorEdited.CanSlam` true _asabp_tailor_edited))
  (:`Released`
    (bind _asabp_tailor_edited_2 (cast `/Game/Characters/ABP_TailorEdited` _returnvalue))
    (set `/Game/Characters/ABP_TailorEdited.CanSlam` false _asabp_tailor_edited_2)))

(event `Punch`
  (bind _returnvalue (`self.K2_GetActorLocation` self))
  ;[1 1 1] Deal Punch Damage
  (bind (_outhit _returnvalue_2) (`KismetSystemLibrary.CapsuleTraceSingleByProfile` _returnvalue (+ _returnvalue (* (`self.GetActorForwardVector` self) (`self.PunchRange`))) 50.0 0.0 "None" false (`|MakeArray` self :!type "Actor Object Reference")))
  (`GameplayStatics.PlaySound2D` "/Game/BeaverFangAudio/fx/atk/crunch.crunch" 1.0 1.0 0.0 null null)
  (if _returnvalue_2
    (for _array_element (`|MakeArray` _outhit)
      (`GameplayStatics.ApplyDamage` (`.HitActor` (`GameplayStatics.BreakHitResult` _array_element)) (`self.PunchDamage`)))))

(event `Slam`
  (bind _returnvalue (+ (`self.K2_GetActorLocation` self) (* (`self.GetActorForwardVector` self) (`self.SlamRange`))))
  ;[1 1 1] Deal Slam Damage
  (bind _outhit (`KismetSystemLibrary.CapsuleTraceSingleByProfile` _returnvalue _returnvalue 60.0 0.0 "None" false (`|MakeArray` self :!type "Actor Object Reference")))
  (`GameplayStatics.PlaySound2D` "/Game/BeaverFangAudio/fx/atk/whap.whap" 1.0 1.0 0.0 null null)
  (if true
    (for _array_element (`|MakeArray` _outhit)
      (`GameplayStatics.ApplyDamage` (`.HitActor` (`GameplayStatics.BreakHitResult` _array_element)) (`self.SlamDamage`)))))

(event `self.ReceiveAnyDamage`
  (params (Damage :type "Float (single-precision)") (DamageType :type "DamageType Object Reference") (InstigatedBy :type "Controller Object Reference") (DamageCauser :type "Actor Object Reference"))
  (bind _returnvalue (`GameplayStatics.GetPlayerController` 0))
  ;[1 1 1] Take Damage
  (`GameplayStatics.PlaySound2D` "/Game/BeaverFangAudio/fx/eep/squeak.squeak" 1.0 1.0 0.0 null null)
  (bind _output_get (set `self.CurrentHealth` (- (`self.CurrentHealth`) Damage)))
  (if (<= _output_get 0.0)
    (bind _returnvalue_2 (`|CreateWidget` "/Game/Widgets/Game_Menus/Player2_Victory.Player2_Victory_C"))
    (`UserWidget.AddToViewport` _returnvalue_2 0)
    (`self.DisableInput` (`GameplayStatics.GetPlayerCharacter` 0) _returnvalue)
    (`self.DisableInput` (`GameplayStatics.GetPlayerCharacter` 1) _returnvalue)
    (set `PlayerController.bShowMouseCursor` true _returnvalue)
    (`GameplayStatics.SetGamePaused` true)))

(event `self.ReceiveBeginPlay`
  (set `self.CurrentHealth` (`self.MaxHealth`)))

(fn `CalculateDead`
  (if (<= (`self.Health`) 0.0)
    (set `self.isDead` true)
    (else
      (set `self.isDead` false))))

(fn `CalculateHealth`
  (params (Delta :type "Float (double-precision)"))
  (set `self.Health` (+ Delta (`self.Health`)))
  (`self.CalculateDead`))

(fn `UserConstructionScript`)